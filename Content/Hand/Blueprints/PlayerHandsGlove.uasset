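; Player glove actor that shows the left and right hand meshes and manages their capsule collision from HandManager state.
; On BeginPlay it passes the owning HandManager to both glove anim instances and caches the HandPlayerController.
; Each tick it toggles each glove's visibility and component ticking from the manager's visibility flags.
; When accepted-angle state changes, it switches child capsules between query-only and no collision and notifies the controller.
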(event EventBeginPlay
  (bind _asleft_glove_anim (Utilities|Casting|CastToLeftGlove_Anim (Components|SkeletalMesh|GetAnimInstance (Variables|Default|GetLeft)))
    (:then
      (bind _ashand_manager (Utilities|Casting|CastToHandManager (Components|GetOwner)))
      (Variables|/Game/Hand/Blueprints/Glove/LeftGlove_Anim.LeftGlove_Anim_C|SetHandManager _asleft_glove_anim _ashand_manager)
      (bind _asright_glove_anim (Utilities|Casting|CastToRightGlove_Anim (Components|SkeletalMesh|GetAnimInstance (Variables|Default|GetRight)))
        (:then
          (Variables|/Game/Hand/Blueprints/Glove/RightGlove_Anim.RightGlove_Anim_C|SetHandManager _asright_glove_anim _ashand_manager)
          (Variables|Default|SetHand%20Manager _ashand_manager)
          (bind _ashand_player_controller (Utilities|Casting|CastToHandPlayerController (Game|GetPlayerController 0)))
          (Variables|Default|SetHandPlayerController _ashand_player_controller))
        (:CastFailed
          (Development|PrintString "anim instance cast fail"))))
    (:CastFailed
      (Development|PrintString "anim instance cast fail"))))

(event EventTick
  (params (DeltaSeconds :type Float%20%28single-precision%29))
  (bind _hand_manager (Variables|Default|GetHand%20Manager))
  (bind _left (Variables|Default|GetLeft))
  (bind _right (Variables|Default|GetRight))
  (bind _returnvalue (Class|ActorComponent|IsComponentTickEnabled _right))
  (bind _returnvalue_2 (Class|ActorComponent|IsComponentTickEnabled _left))
  (CallFunction|SetAngleCapsuleCollision)
  ;[1 1 1] Left Visible
  (if (Variables|/Game/Hand/Blueprints/HandManager.HandManager_C|GetLeftVisible _hand_manager)
    (if _returnvalue_2
      _
      (else
        (Components|Tick|SetComponentTickEnabled _left true)
        (Rendering|SetVisibility _left true true)))
    (elif _returnvalue_2
      (Components|Tick|SetComponentTickEnabled _left false)
      (Rendering|SetVisibility _left false true)))
  ;[1 1 1] Right visible
  (if (Variables|/Game/Hand/Blueprints/HandManager.HandManager_C|GetRightVisible _hand_manager)
    (if (not _returnvalue)
      (Components|Tick|SetComponentTickEnabled _right true)
      (Rendering|SetVisibility _right true true))
    (elif _returnvalue
      (Components|Tick|SetComponentTickEnabled _right false)
      (Rendering|SetVisibility _right false true))))

(fn ConstructionScript)

(fn SetAngleCapsuleCollision
  (bind _hand_manager (Variables|Default|GetHand%20Manager))
  (bind _acceptedangles (Variables|/Game/Hand/Blueprints/HandManager.HandManager_C|GetAcceptedAngles _hand_manager))
  (if (and _acceptedangles (Variables|Default|GetCapsules%20Disabled))
    (for _array_element (Components|GetChildrenComponents (Variables|Default|GetLeft) false)
      (bind _ascapsule_collision (Utilities|Casting|CastToCapsuleComponent _array_element))
      (Collision|SetCollisionEnabled _ascapsule_collision "QueryOnly")
      (bind _output_get (Variables|Default|SetCapsules%20Disabled false))
      (Default|AcceptedAnglesCapsule (Variables|Default|GetHandPlayerController) _output_get))
    (for _array_element_2 (Components|GetChildrenComponents (Variables|Default|GetRight) false)
      (bind _ascapsule_collision_2 (Utilities|Casting|CastToCapsuleComponent _array_element_2))
      (Collision|SetCollisionEnabled _ascapsule_collision_2 "QueryOnly")
      (bind _output_get_2 (Variables|Default|SetCapsules%20Disabled false))
      (Default|AcceptedAnglesCapsule (Variables|Default|GetHandPlayerController) _output_get_2))
    (elif (and (not _acceptedangles) (not (Variables|Default|GetCapsules%20Disabled)))
      (for _array_element_3 (Components|GetChildrenComponents (Variables|Default|GetLeft) false)
        (bind _ascapsule_collision_3 (Utilities|Casting|CastToCapsuleComponent _array_element_3))
        (Collision|SetCollisionEnabled _ascapsule_collision_3 "NoCollision")
        (bind _output_get_3 (Variables|Default|SetCapsules%20Disabled true))
        (Default|AcceptedAnglesCapsule (Variables|Default|GetHandPlayerController) _output_get_3))
      (for _array_element_4 (Components|GetChildrenComponents (Variables|Default|GetRight) false)
        (bind _ascapsule_collision_4 (Utilities|Casting|CastToCapsuleComponent _array_element_4))
        (Collision|SetCollisionEnabled _ascapsule_collision_4 "NoCollision")
        (bind _output_get_4 (Variables|Default|SetCapsules%20Disabled true))
        (Default|AcceptedAnglesCapsule (Variables|Default|GetHandPlayerController) _output_get_4)))))