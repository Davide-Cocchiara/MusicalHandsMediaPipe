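; MediaPipe holistic tracking Blueprint that visualizes pose, face, hand, eye and iris landmarks.
; It starts the pipeline on BeginPlay and stops it on EndPlay.
; Each Tick it draws the camera origin, then each observer's landmarks relative to that origin, color-coded by body part, with larger primitives for the pose.
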(event EventBeginPlay
  (CallFunction|StartPipeline))

(event EventTick
  (params (DeltaSeconds :type Float%20%28single-precision%29))
  (bind _cameraorigin (Variables|Default|GetCameraOrigin))
  (CallFunction|DrawCameraOrigin)
  (CallFunction|DrawLandmarks (Variables|Default|GetPose) 0 _cameraorigin 6.0 "(R=1.000000,G=1.000000,B=0.000000,A=1.000000)")
  (CallFunction|DrawLandmarks (Variables|Default|GetFace) 0 _cameraorigin 4.0 "(R=0.000000,G=1.000000,B=0.000000,A=1.000000)")
  (CallFunction|DrawLandmarks (Variables|Default|GetHandL) 0 _cameraorigin 4.0 "(R=0.000000,G=0.000000,B=1.000000,A=1.000000)")
  (CallFunction|DrawLandmarks (Variables|Default|GetHandR) 0 _cameraorigin 4.0 "(R=0.000000,G=0.000000,B=1.000000,A=1.000000)")
  (CallFunction|DrawLandmarks (Variables|Default|GetEyeL) 0 _cameraorigin 4.0 "(R=0.000000,G=0.000000,B=1.000000,A=1.000000)")
  (CallFunction|DrawLandmarks (Variables|Default|GetEyeR) 0 _cameraorigin 4.0 "(R=0.000000,G=0.000000,B=1.000000,A=1.000000)")
  (CallFunction|DrawLandmarks (Variables|Default|GetIrisL) 0 _cameraorigin 4.0 "(R=1.000000,G=0.000000,B=0.000000,A=1.000000)")
  (CallFunction|DrawLandmarks (Variables|Default|GetIrisR) 0 _cameraorigin 4.0 "(R=1.000000,G=0.000000,B=0.000000,A=1.000000)"))

(event EventEndPlay
  (params (EndPlayReason :type EEndPlayReason%20Enum :default "Destroyed"))
  (CallFunction|StopPipeline))

(fn ConstructionScript)