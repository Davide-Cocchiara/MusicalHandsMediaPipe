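; MediaPipe Blueprint that visualizes detected 3D pose landmarks in the world as debug drawing.
; On BeginPlay it resets the pipeline's graph nodes to a single node and starts the pipeline, then stops it on EndPlay.
; Each tick it draws the world origin and, when the PoseWorld observer has detections, the landmarks offset from that origin.
; A red debug box highlights the first landmark.
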(event EventBeginPlay
  (bind _pipeline (Variables|Default|GetPipeline))
  (bind _graphnodes (Variables|/Script/MediaPipe.MediaPipePipelineComponent|GetGraphNodes _pipeline))
  (Utilities|Array|Clear _graphnodes)
  (Utilities|Array|Add _graphnodes (Variables|MediaPipe|Pipeline|GetGraphNode))
  (CallFunction|StartPipeline))

(event EventTick
  (params (DeltaSeconds :type Float%20%28single-precision%29))
  (bind _poseworld (Variables|Default|GetPoseWorld))
  (CallFunction|DrawWorldOrigin)
  (if (Class|MediaPipeObserverComponent|HaveDetections _poseworld)
    (CallFunction|DrawLandmarks _poseworld 0 (Variables|Default|GetWorldOrigin) 6.0 "(R=1.000000,G=1.000000,B=0.000000,A=1.000000)")
    (Rendering|Debug|DrawDebugBox (+ (.Pos (Utilities|Struct|BreakMediaPipeLandmark (Class|MediaPipeLandmarkObserverComponent|GetLandmark (Variables|Default|GetPoseWorld)))) (Variables|Default|GetWorldOrigin)) "2.000000,2.000000,2.000000" "(R=1.000000,G=0.000000,B=0.000000,A=1.000000)" "0, 0, 0" 0.0 0.0)))

(event EventEndPlay
  (params (EndPlayReason :type EEndPlayReason%20Enum :default "Destroyed"))
  (CallFunction|StopPipeline))

(fn ConstructionScript)