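; MediaPipe puppet avatar that drives a fully physics-simulated skeletal mesh from detected pose landmarks.
; On BeginPlay it creates one physics handle per landmark-to-bone mapping entry, grabs that bone, then starts the MediaPipe pipeline.
; Each tick with detections, it draws debug landmarks and moves handles of sufficiently present landmarks to their positions, reapplying damping and stiffness so the body follows like a marionette.
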(event EventBeginPlay
  (bind _pipeline (Variables|Default|GetPipeline))
  (bind _graphnodes (Variables|/Script/MediaPipe.MediaPipePipelineComponent|GetGraphNodes _pipeline))
  (CallFunction|InitGrabbers)
  (Utilities|Array|Clear _graphnodes)
  (Utilities|Array|Add _graphnodes (Variables|MediaPipe|Pipeline|GetGraphNode))
  (CallFunction|StartPipeline))

(event EventTick
  (params (DeltaSeconds :type Float%20%28single-precision%29))
  (bind _pose (Variables|Default|GetPose))
  (CallFunction|DrawWorldOrigin)
  (if (Class|MediaPipeObserverComponent|HaveDetections _pose)
    (CallFunction|DrawLandmarks _pose 0 (Variables|Default|GetWorldOrigin) 6.0 "(R=1.000000,G=1.000000,B=0.000000,A=1.000000)")
    (Rendering|Debug|DrawDebugBox (+ (.Pos (Utilities|Struct|BreakMediaPipeLandmark (Class|MediaPipeLandmarkObserverComponent|GetLandmark (Variables|Default|GetPose)))) (Variables|Default|GetWorldOrigin)) "2.000000,2.000000,2.000000" "(R=1.000000,G=0.000000,B=0.000000,A=1.000000)" "0, 0, 0" 0.0 0.0)
    (CallFunction|UpdateGrabbers)))

(event EventEndPlay
  (params (EndPlayReason :type EEndPlayReason%20Enum :default "Destroyed"))
  (CallFunction|StopPipeline))

(fn ConstructionScript)

(fn InitGrabbers
  (bind _avatar (Variables|Default|GetAvatar))
  (Class|SkeletalMeshComponent|SetAllBodiesSimulatePhysics (Variables|Default|GetAvatar) true)
  (for _array_element (Variables|MediaPipe|Avatar|GetMapping)
    (bind _returnvalue (Game|AddComponentbyClass "/Script/Engine.PhysicsHandleComponent"))
    (Utilities|Map|Add (Variables|MediaPipe|Avatar|GetGrabbers) (.LandmarkId (Utilities|Struct|BreakMP_BoneMapping _array_element)) _returnvalue)
    (Class|PhysicsHandleComponent|GrabComponentatLocation _returnvalue _avatar (.AvatarBoneName (Utilities|Struct|BreakMP_BoneMapping _array_element)) (Transformation|GetSocketLocation _avatar (.AvatarBoneName (Utilities|Struct|BreakMP_BoneMapping _array_element))))
    (Physics|Components|PhysicsHandle|SetTargetLocation _returnvalue (Transformation|GetSocketLocation _avatar (.AvatarBoneName (Utilities|Struct|BreakMP_BoneMapping _array_element))))))

(fn UpdateGrabbers
  (for _array_element (Variables|MediaPipe|Avatar|GetMapping)
    (if (> (.Presence (Utilities|Struct|BreakMediaPipeLandmark (Class|MediaPipeLandmarkObserverComponent|GetLandmark (Variables|Default|GetPose) 0 (.LandmarkId (Utilities|Struct|BreakMP_BoneMapping _array_element))))) 0.5)
      (Physics|Components|PhysicsHandle|SetTargetLocation (.Value (Utilities|Map|Find (Variables|MediaPipe|Avatar|GetGrabbers) (.LandmarkId (Utilities|Struct|BreakMP_BoneMapping _array_element)))) (.Pos (Utilities|Struct|BreakMediaPipeLandmark (Class|MediaPipeLandmarkObserverComponent|GetLandmark (Variables|Default|GetPose) 0 (.LandmarkId (Utilities|Struct|BreakMP_BoneMapping _array_element))))))
      (Class|PhysicsHandleComponent|SetLinearDamping (.Value (Utilities|Map|Find (Variables|MediaPipe|Avatar|GetGrabbers) (.LandmarkId (Utilities|Struct|BreakMP_BoneMapping _array_element)))) (Variables|MediaPipe|Avatar|GetLinearDamping))
      (Class|PhysicsHandleComponent|SetLinearStiffness (.Value (Utilities|Map|Find (Variables|MediaPipe|Avatar|GetGrabbers) (.LandmarkId (Utilities|Struct|BreakMP_BoneMapping _array_element)))) (Variables|MediaPipe|Avatar|GetLinearStiffness))
      (Class|PhysicsHandleComponent|SetAngularDamping (.Value (Utilities|Map|Find (Variables|MediaPipe|Avatar|GetGrabbers) (.LandmarkId (Utilities|Struct|BreakMP_BoneMapping _array_element)))) (Variables|MediaPipe|Avatar|GetAngularDamping))
      (Class|PhysicsHandleComponent|SetAngularStiffness (.Value (Utilities|Map|Find (Variables|MediaPipe|Avatar|GetGrabbers) (.LandmarkId (Utilities|Struct|BreakMP_BoneMapping _array_element)))) (Variables|MediaPipe|Avatar|GetAngularStiffness)))))

(fn GetLandmarkPos
  (params (LandmarkId :type Integer))
  (bind _pose (Variables|Default|GetPose))
  (bind _returnvalue (Class|MediaPipeLandmarkObserverComponent|GetLandmark _pose 0 LandmarkId))
  (bind (_pos _visibility _presence) (Utilities|Struct|BreakMediaPipeLandmark _returnvalue))
  (return _pos _presence))