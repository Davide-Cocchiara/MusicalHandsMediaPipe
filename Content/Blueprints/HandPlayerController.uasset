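; Player controller for hand-played instruments that spawns the HandManager and two HUD widgets for the local player.
; It forwards finger, hand-placement and mode-text events to HandStatus, and keys start the video, toggle arpeggiator/melody or open the main menu.
; ChangeInstrument either sets melody mode or flips the key between C and G, depending on the current instrument.
; Helpers read the first OSCFingerPluck actor and write to all; key changes also reach HandPlayerPawn.
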(event Custom|PlayedNoteFinger
  (params (Finger :type String))
  (Default|DisplayNotePlayedFinger (Variables|Default|GetHandWidget) Finger))

(event Custom|AcceptedAnglesCapsule
  (params (Capsules%20Disabled :type Boolean))
  (Default|ShowHidePlaceHands (Variables|Default|GetHandWidget) Capsules%20Disabled))

(event Custom|SetModeText
  (params (ModeText :type Text))
  (Default|SetModeText (Variables|Default|GetHandWidget) ModeText))

(event Custom|Change%20Instrument
  (bind _currinstrument (CallFunction|GetCurrentInstrument))
  (if (< _currinstrument 4)
    (CallFunction|SwitchModeasMelody)
    (else
      (bind _curr_key (CallFunction|GetCurrentKey))
      (switch int _curr_key ; 0 is C, 1 is G
        (:0
          (CallFunction|NewKeytoInstruments 1)
          (CallFunction|SendNewKey 1 self))
        (:1
          (CallFunction|NewKeytoInstruments)
          (CallFunction|SendNewKey 0 self))))))

(event Custom|SendNewKey
  (params (NewKey :type Byte) (Player%20Controller :type Player%20Controller%20Object%20Reference))
  (bind _ashand_player_pawn (Utilities|Casting|CastToHandPlayerPawn (Game|Player|GetPlayerPawn 0)))
  (Default|ApplyNewKey _ashand_player_pawn NewKey Player%20Controller))

(event EventBeginPlay
  (bind _returnvalue (Game|GetPlayerController 0))
  (if (not (Networking|IsDedicatedServer))
    (if (Pawn|IsLocalController)
      (Game|SpawnActorfromClass "/Game/Hand/Blueprints/HandManager.HandManager_C" (Math|Transform|MakeTransform "0, 0, 0") "Undefined" _returnvalue 0)
      (bind _returnvalue_2 (UserInterface|CreateWidget "/Game/Blueprints/HandStatus.HandStatus_C" _returnvalue))
      (bind _output_get (Variables|Default|SetHandWidget _returnvalue_2))
      (UserInterface|Viewport|AddtoViewport _output_get 0)
      (bind _returnvalue_3 (UserInterface|CreateWidget "/Game/Video/FattoriaWidget.FattoriaWidget_C" _returnvalue))
      (bind _output_get_2 (Variables|Default|SetVideoWidget _returnvalue_3))
      (UserInterface|Viewport|AddtoViewport _output_get_2 0))))

(event EventTick
  (params (DeltaSeconds :type Float%20%28single-precision%29)))

(event Input|KeyboardEvents|E
  (params (Key :type Key%20Structure :default "None"))
  (:Pressed
    (Default|StartVideo (Variables|Default|GetVideoWidget))
    (CameraShake|Start (Variables|Default|GetMediaSound))))

(event Input|KeyboardEvents|Escape
  (params (Key :type Key%20Structure :default "None"))
  (:Pressed
    (Game|OpenLevel(byObjectReference) "/Game/Maps/MainMenu.MainMenu")))

(event Input|KeyboardEvents|Tab
  (params (Key :type Key%20Structure :default "None"))
  (:Pressed
    (CallFunction|SwitchArpeggiatorMelody)))

(event Input|KeyboardEvents|SpaceBar
  (params (Key :type Key%20Structure :default "None")))

(fn ConstructionScript)

(fn NewKeytoInstruments
  (params (New%20Key :type Integer))
  (bind _outactors (Actor|GetAllActorsOfClass "/Game/OSC/Instruments/OSCFingerPluck.OSCFingerPluck_C"))
  (for _array_element _outactors
    (Default|SetNewKey _array_element New%20Key)))

(fn GetCurrentKey
  (bind _outactors (Actor|GetAllActorsOfClass "/Game/OSC/Instruments/OSCFingerPluck.OSCFingerPluck_C"))
  (for _array_element _outactors
    (bind _currkey (Default|GetCurrentKey _array_element))
    (return _currkey))
  (return -1))

(fn GetCurrentInstrument
  (bind _outactors (Actor|GetAllActorsOfClass "/Game/OSC/Instruments/OSCFingerPluck.OSCFingerPluck_C"))
  (for _array_element _outactors
    (bind _currinstr (Default|GetCurrentInstrument _array_element))
    (return _currinstr))
  (return -1))

(fn SwitchModeasMelody
  (bind _outactors (Actor|GetAllActorsOfClass "/Game/OSC/Instruments/OSCFingerPluck.OSCFingerPluck_C"))
  (for _array_element _outactors
    (Default|ChangeModeasMelody _array_element)))

(fn SwitchArpeggiatorMelody
  (bind _outactors (Actor|GetAllActorsOfClass "/Game/OSC/Instruments/OSCFingerPluck.OSCFingerPluck_C"))
  (for _array_element _outactors
    (Default|SwitchArpeggiatorMelody _array_element)))