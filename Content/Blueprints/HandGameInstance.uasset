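; Game instance for a hand game that handles the main menu and launching solo or multiplayer play.
; ShowMainMenu creates and reuses the menu widget and shows the cursor.
; HostGame creates a session with configurable player count and LAN flag, then opens FingerPluck as a listen server, while SoloGame opens it without that option.
; JoinGame builds an "open" console command from the supplied IP and port; a second session-creation chain sits unconnected.
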(event Custom|ShowMainMenu
  (bind _returnvalue (Game|GetPlayerController 0))
  ;[1 1 1] Main Menu
  (Utilities|IsValid (Variables|Default|GetMain%20Menu)
    (:Is%20Valid
      _)
    (:Is%20Not%20Valid
      (bind _returnvalue_2 (UserInterface|CreateWidget "/Game/Blueprints/MainMenu.MainMenu_C" _returnvalue))
      (bind _output_get (Variables|Default|SetMain%20Menu _returnvalue_2))))
  (UserInterface|Viewport|AddtoViewport _output_get 0)
  (Variables|/Script/Engine.PlayerController|SetbShowMouseCursor _returnvalue true))

(event Custom|Host%20Game
  ;[1 1 1] Host Game
  (|Session (Game|GetPlayerController 0) (Variables|Default|GetMax%20Players) (Variables|Default|GetLAN) ; Public connections: Max players
    (:OnSuccess
      (Game|OpenLevel(byObjectReference) "/Game/MusicRooms/FingerPluck.FingerPluck" true "listen"))
    (:OnFailure
      (Development|PrintString "ERROR In hosting game"))))

(event Custom|Solo%20Game
  ;[1 1 1] Solo
  (Game|OpenLevel(byObjectReference) "/Game/MusicRooms/FingerPluck.FingerPluck"))

(event Custom|Join%20Game
  (params (IP%20and%20Port :type String))
  ;[1 1 1] Join game
  (Development|ExecuteConsoleCommand (Utilities|String|Append "open " IP%20and%20Port) (Game|GetPlayerController 0)))